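; BP_Mom is a Mom actor that turns to face the player and shows its name when a raycast hits it.
; Tick rotates it on yaw only toward the player camera, like an upright billboard.
; The construction script fills the name text component from the Name variable and clears IsNameVisible.
; OnRaycastHit makes that text visible, while OnRaycastRemove only defers to the parent implementation.
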(event EventTick
  (params (DeltaSeconds :type Float%20%28single-precision%29))
  ;[1 1 1] Always facing the PlayerCharacter
  (Transformation|SetActorRotation (Math|Rotator|MakeRotator 0.0 0.0 (.Yaw (Math|Rotator|BreakRotator (Math|Rotator|FindLookatRotation (Transformation|GetActorLocation) (Transformation|GetActorLocation (Game|GetPlayerCameraManager 0))))))))

(fn ConstructionScript
  (Rendering|Components|TextRender|SetText (Variables|Default|GetTXT_CharacterName) (Utilities|Text|ToText(String) (Variables|Default|GetName)))
  (Variables|Default|SetisNameVisible false))

(fn OnRaycastHit
  (Rendering|SetVisibility (Variables|Default|GetTXT_CharacterName) true false))

(fn OnRaycastRemove
  (|CallParentFunction))