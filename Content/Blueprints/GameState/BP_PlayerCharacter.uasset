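; BP_PlayerCharacter is the player character, handling Enhanced Input movement and look, plus interaction with world objects.
; Tick line-traces toward the camera's forward view and calls raycast hit and remove events on interactable BP_ObjBase actors for highlighting.
; Interact repeats the trace, then opens dialogue or sends InteractMessage for switches and chores, with later presses advancing dialogue.
; BeginPlay creates the chore and dialogue widgets, and a toggle input controls the chore list.
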(event Input|EnhancedActionEvents|EnhancedInputActionIA_Interact
  (params (ActionValue :type Boolean) (ElapsedSeconds :type Float%20%28double-precision%29) (TriggeredSeconds :type Float%20%28double-precision%29) (InputAction :type Input%20Action%20Object%20Reference :default "/Game/Input/Actions/IA_Interact.IA_Interact"))
  (bind _returnvalue (Game|GetPlayerCameraManager 0))
  (bind _dialoguewidget (Variables|Default|GetDialogueWidget))
  (:Started
    (if (Variables|Default|GetInDialogue)
      (bind _result (Math|Integer|IncrementInt (Variables|Default|GetDialogueIndex))
        (:%20%20
          (if (>= (Variables|Default|GetDialogueIndex) (Utilities|Array|Length (Variables|/Game/Blueprints/GameState/V2/BP_ObjBase.BP_ObjBase_C|GetDialogueText (Variables|Default|GetInteractionInstigator))))
            (Default|RemoveDialogueUI _dialoguewidget)
            (Variables|Default|SetInDialogue false)
            (else
              (Default|ProgressDialogue _dialoguewidget (Utilities|Array|Get(acopy) (Variables|/Game/Blueprints/GameState/V2/BP_ObjBase.BP_ObjBase_C|GetDialogueText (Variables|Default|GetInteractionInstigator)) _result))))))
      (else
        (bind _outhit (Collision|LineTraceByChannel (Transformation|GetActorLocation) (+ (Transformation|GetActorLocation _returnvalue) (* (Transformation|GetActorForwardVector _returnvalue) (Variables|Default|GetRaycastDistance))) "TraceTypeQuery1" false 0 "ForOneFrame"))
        (bind _output_get (Variables|Default|SetInteractedObject (.HitActor (Collision|BreakHitResult _outhit))))
        (if (Utilities|DoesObjectImplementInterface _output_get "/Game/Blueprints/GameState/V2/BPI_Interactable.BPI_Interactable_C")
          (bind _asbp_obj_base (Utilities|Casting|CastToBP_ObjBase _output_get)
            (:then
              (bind _output_get_2 (Variables|Default|SetInteractionInstigator _asbp_obj_base))
              (if (Utilities|Enum|Equal(Enum) (Variables|/Game/Blueprints/GameState/V2/BP_ObjBase.BP_ObjBase_C|GetInteractionType _output_get_2) "NewEnumerator1") ; If interaction is dialogue
                (Variables|Default|SetInDialogue true)
                (Variables|Default|SetDialogueIndex 0)
                (Default|ShowDialogueUI (Variables|Default|GetDialogueWidget) "/Game/Assets/Oofers/Komaeda.Komaeda" (Utilities|Array|Get(acopy) (Variables|/Game/Blueprints/GameState/V2/BP_ObjBase.BP_ObjBase_C|GetDialogueText (Variables|Default|GetInteractionInstigator))) (Variables|/Game/Blueprints/GameState/V2/BP_ObjBase.BP_ObjBase_C|GetDialogueName (Variables|Default|GetInteractionInstigator)))
                (elif (Utilities|Enum|Equal(Enum) (Variables|/Game/Blueprints/GameState/V2/BP_ObjBase.BP_ObjBase_C|GetInteractionType _output_get_2) "NewEnumerator2") ; If interaction is a switch (lights, doors)
                  (Class|BPIInteractable|Interact(Message) (Variables|Default|GetInteractionInstigator))
                  (elif (Utilities|Enum|Equal(Enum) (Variables|/Game/Blueprints/GameState/V2/BP_ObjBase.BP_ObjBase_C|GetInteractionType _output_get_2) "NewEnumerator0") ; If interaction is a Chore
                    (Class|BPIInteractable|Interact(Message) (Variables|Default|GetInteractionInstigator))))))
            (:CastFailed
              (Development|PrintString "Cast Failed!"))))))))

(event Input|EnhancedActionEvents|EnhancedInputActionIA_Move
  (params (ActionValue :type Vector%202D%20Structure) (ElapsedSeconds :type Float%20%28double-precision%29) (TriggeredSeconds :type Float%20%28double-precision%29) (InputAction :type Input%20Action%20Object%20Reference :default "/Game/Input/Actions/IA_Move.IA_Move"))
  ;[1 1 1] Moement Controls
  ;;[1 1 1] Left/Right Movement
  (Pawn|Input|AddMovementInput (Math|Vector|GetRightVector (Pawn|GetControlRotation :!class /Script/Engine.Pawn)) (.x ActionValue) false)
  ;;[1 1 1] Forward/Backward Movement
  (Pawn|Input|AddMovementInput (Math|Vector|GetForwardVector (Pawn|GetControlRotation :!class /Script/Engine.Pawn)) (.y ActionValue) false))

(event Input|EnhancedActionEvents|EnhancedInputActionIA_Look
  (params (ActionValue :type Vector%202D%20Structure) (ElapsedSeconds :type Float%20%28double-precision%29) (TriggeredSeconds :type Float%20%28double-precision%29) (InputAction :type Input%20Action%20Object%20Reference :default "/Game/Input/Actions/IA_Look.IA_Look"))
  ;[1 1 1] Camera Controls
  (Pawn|Input|AddControllerYawInput (.x ActionValue))
  (Pawn|Input|AddControllerPitchInput (* (.y ActionValue) (Variables|Default|GetPitchSensitivity))))

(event Input|EnhancedActionEvents|EnhancedInputActionIA_ToggleObjective
  (params (ActionValue :type Boolean) (ElapsedSeconds :type Float%20%28double-precision%29) (TriggeredSeconds :type Float%20%28double-precision%29) (InputAction :type Input%20Action%20Object%20Reference :default "/Game/Input/IA_ToggleObjective.IA_ToggleObjective"))
  ;[1 1 1] Tab to open chorelist.
  (Default|ToggleObjective (Variables|Default|GetChoreWidget)))

(event EventBeginPlay
  ;[1 1 1] Add Input System
  (bind _asplayer_controller (Utilities|Casting|CastToPlayerController (Pawn|GetController)))
  (Utilities|IsValid (PlayerController|LocalPlayerSubsystems|GetEnhancedInputLocalPlayerSubsystem _asplayer_controller)
    (:Is%20Valid
      (Input|AddMappingContext (PlayerController|LocalPlayerSubsystems|GetEnhancedInputLocalPlayerSubsystem _asplayer_controller) "/Game/Input/IMC_default.IMC_default" 0 "(bIgnoreAllPressedKeysUntilRelease=True,bForceImmediately=False,bNotifyUserSettings=False)")
      (bind _returnvalue (UserInterface|CreateWidget "/Game/UI/W_Chores.W_Chores_C"))
      (bind _output_get (Variables|Default|SetChoreWidget _returnvalue))
      (UserInterface|Viewport|AddtoViewport _output_get 0)
      (Widget|SetRenderOpacity (Variables|Default|GetChoreWidget) 0.0)
      (bind _returnvalue_2 (UserInterface|CreateWidget "/Game/UI/W_Dialogue.W_Dialogue_C"))
      (bind _output_get_2 (Variables|Default|SetDialogueWidget _returnvalue_2))
      (Variables|/Script/UMG.Widget|SetVisibility _output_get_2 "Hidden")
      (UserInterface|Viewport|AddtoViewport _output_get_2 0)
      (Default|CallOnReady))))

(event EventTick
  (params (DeltaSeconds :type Float%20%28single-precision%29))
  (bind _returnvalue (Game|GetPlayerCameraManager 0))
  ;[1 1 1] Highlights when we go near Interactable things.
  (bind _outhit (Collision|LineTraceByChannel (Transformation|GetActorLocation) (+ (Transformation|GetActorLocation _returnvalue) (* (Transformation|GetActorForwardVector _returnvalue) (Variables|Default|GetRaycastDistance))) "TraceTypeQuery1" false 0 "ForOneFrame"))
  (if (!= (Variables|Default|GetLookingAtObject) (.HitActor (Collision|BreakHitResult _outhit)))
    (bind _asbp_obj_base (Utilities|Casting|CastToBP_ObjBase (Variables|Default|GetLookingAtObject))
      (:then
        (Default|OnRaycastRemove _asbp_obj_base)
        (Variables|Default|SetLookingAtObject (.HitActor (Collision|BreakHitResult _outhit))))
      (:CastFailed
        (Variables|Default|SetLookingAtObject (.HitActor (Collision|BreakHitResult _outhit)))))
    (elif (Utilities|DoesObjectImplementInterface (.HitActor (Collision|BreakHitResult _outhit)) "/Game/Blueprints/GameState/V2/BPI_Interactable.BPI_Interactable_C")
      (bind _asbp_obj_base_2 (Utilities|Casting|CastToBP_ObjBase (.HitActor (Collision|BreakHitResult _outhit))))
      (Default|OnRaycastHit _asbp_obj_base_2))))

(fn ConstructionScript)