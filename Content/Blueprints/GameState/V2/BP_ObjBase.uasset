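; BP_ObjBase is an object base Blueprint that shows a text name label while the object is targeted by a raycast.
; The construction script fills TXTCharacterName from the Name variable and sets IsNameVisible to false.
; OnRaycastHit and OnRaycastRemove show and hide the label directly, without reading or updating that flag.
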(fn ConstructionScript
  (Rendering|Components|TextRender|SetText (Variables|Default|GetTXT_CharacterName) (Utilities|Text|ToText(String) (Variables|Default|GetName)))
  (Variables|Default|SetisNameVisible false))

(fn OnRaycastHit
  (Rendering|SetVisibility (Variables|Default|GetTXT_CharacterName) true false))

(fn OnRaycastRemove
  (Rendering|SetVisibility (Variables|Default|GetTXT_CharacterName) false false))