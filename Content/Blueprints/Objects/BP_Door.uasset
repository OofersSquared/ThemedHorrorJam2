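; BP_Door is an interactable door that toggles open and closed with a timeline-driven 90-degree yaw swing.
; Interact plays or reverses the timeline based on IsOpen, ignoring calls while animating and flipping the state on finish.
; Each update rotates the door and its separate collision component, also nudging the collision by a fixed per-tick offset whose direction depends on IsOpen.
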(event EventInteract
  (bind _doorcollision (Variables|Default|GetDoorCollision))
  (bind _doorcollision_2 (Variables|Default|GetDoorCollision))
  ;[1 1 1] Door opening code
  (if (not (Variables|Default|GetisAnimating))
    (Variables|Default|SetisAnimating true)
    (if (Variables|Default|GetisOpen)
      (bind _doorrotation (Timeline|Timeline Reverse)
        (:Update
          (Transformation|SetRelativeRotation (Variables|Default|GetDoor) (Math|Rotator|Lerp(Rotator) "0, 0, 0" "0.000000,-90.000000,0.000000" _doorrotation) false false)
          (if (Variables|Default|GetisOpen)
            (Transformation|AddRelativeLocation _doorcollision "2.400000,-1.900000,0.000000" false false)
            (Transformation|SetRelativeRotation _doorcollision (Math|Rotator|Lerp(Rotator) "0, 0, 0" "0.000000,-90.000000,0.000000" _doorrotation) false false)
            (else
              (Transformation|AddRelativeLocation _doorcollision_2 "-2.400000,1.900000,0.000000" false false)
              (Transformation|SetRelativeRotation _doorcollision_2 (Math|Rotator|Lerp(Rotator) "0, 0, 0" "0.000000,-90.000000,0.000000" _doorrotation) false false))))
        (:Finished
          (Variables|Default|SetisOpen (not (Variables|Default|GetisOpen)))
          (Variables|Default|SetisAnimating false)))
      (else
        (Timeline|Timeline PlayFromStart)))))

(fn ConstructionScript)